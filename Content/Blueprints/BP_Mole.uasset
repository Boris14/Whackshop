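; Whack-a-mole target actor that turns to face the player on BeginPlay, then repeatedly moves vertically with appear and laugh sounds.
; A timeline drives its world Z and triggers the laugh, replaying after a short delay while the mole is alive.
; Die speeds up the timeline, reversing it if early in playback; on finish, the mole plays a hit sound, destroys itself and increments the HUD score.
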(event EventBeginPlay
  (bind _returnvalue (Transformation|GetActorLocation))
  (Utilities|FlowControl|Sequence
    (:then_0
      (Transformation|SetActorRotation (Math|Rotator|MakeRotator 0.0 0.0 (.yaw (Math|Rotator|FindLookatRotation (Transformation|GetActorLocation) (Transformation|GetActorLocation (Game|Player|GetPlayerPawn 0)))))))
    (:then_1
      (bind _z (Timeline|MovementTimeline Play)
        (:Update
          (Transformation|SetActorLocation (Math|Vector|MakeVector (.x _returnvalue) (.y _returnvalue) _z) false false))
        (:Finished
          (if (Variables|Default|GetIsDead)
            (Audio|PlaySoundatLocation "/Game/Assets/Audio/Hit.Hit" (Transformation|GetActorLocation) "0, 0, 0" 1.0 1.0 0.0 0 0 0 0)
            (Actor|DestroyActor)
            (bind _foundwidgets (Widget|GetAllWidgetsOfClass "/Game/Blueprints/WBP_HUD.WBP_HUD_C" true))
            (for _array_element _foundwidgets
              (Default|IncreaseScore _array_element))
            (else
              (Utilities|FlowControl|Delay 1.0)
              (Components|Timeline|PlayfromStart (Variables|Default|GetMovementTimeline)))))
        (:MoleLaugh
          (Audio|PlaySoundatLocation "/Game/Assets/Audio/MoleLaugh.MoleLaugh" (Transformation|GetActorLocation) "0, 0, 0" 1.0 1.0 0.0 0 0 0 0))))
    (:then_3
      (Utilities|FlowControl|Delay 1.0)
      (Audio|PlaySoundatLocation "/Game/Assets/Audio/Appear.Appear" (Transformation|GetActorLocation) "0, 0, 0" 1.0 1.0 0.0 0 0 0 0))))

(event Collision|EventActorBeginOverlap
  (params (OtherActor :type Actor%20Object%20Reference)))

(event EventTick
  (params (DeltaSeconds :type Float%20%28single-precision%29)))

(fn ConstructionScript)

(fn Die
  (bind _movementtimeline (Variables|Default|GetMovementTimeline))
  (Variables|Default|SetIsDead true)
  (Components|Timeline|SetPlayRate _movementtimeline 1e+01)
  (if (<= (Components|Timeline|GetPlaybackPosition _movementtimeline) 2.0)
    (Utilities|String|Reverse _movementtimeline)))