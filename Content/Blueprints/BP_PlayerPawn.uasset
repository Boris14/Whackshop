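; Player pawn for a mole-whacking game, which moves, turns and swings a hammer to kill BP_Mole actors.
; Axis inputs set a movement vector that Tick applies relative to actor rotation without sweep, while yaw turning scales with global time dilation to freeze during pause.
; The strike input plays a non-restartable swing timeline that pitches the hammer, with event tracks playing a sound and enabling StrikeCollision overlaps only during the hit window.
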(event Custom|OnStrikeOverlap
  (params (OverlappedComponent :type Primitive%20Component%20Object%20Reference) (OtherActor :type Actor%20Object%20Reference) (OtherComp :type Primitive%20Component%20Object%20Reference) (OtherBodyIndex :type Integer) (bFromSweep :type Boolean) (SweepResult :type Hit%20Result%20Structure%20%28by%20ref%29))
  (bind _asbp_mole (Utilities|Casting|CastToBP_Mole OtherActor))
  (Default|Die _asbp_mole))

(event EventBeginPlay
  (bind _strikecollision (Variables|Default|GetStrikeCollision))
  (Collision|AssignOnComponentBeginOverlap _strikecollision (delegate Custom|OnStrikeOverlap))
  (Variables|/Script/Engine.PrimitiveComponent|SetbGenerateOverlapEvents _strikecollision false)
  (Components|Timeline|SetPlayRate (Variables|Default|GetHammerSwingTimeline) 3.0))

(event Collision|EventActorBeginOverlap
  (params (OtherActor :type Actor%20Object%20Reference)))

(event EventTick
  (params (DeltaSeconds :type Float%20%28single-precision%29))
  (bind _movementinput (Variables|Default|GetMovementInput))
  (bind _speed (Variables|Default|GetSpeed))
  (bind _returnvalue (* DeltaSeconds _speed _movementinput))
  (Transformation|AddActorWorldOffset (Math|Vector|RotateVector (Math|Vector|MakeVector (.x _returnvalue) (.y _returnvalue) 0.0) (Transformation|GetActorRotation))))

(event Input|ActionEvents|InputActionHammerStrike
  (params (Key :type Key%20Structure :default "None"))
  (bind _hammer (Variables|Default|GetHammer))
  (bind _strikecollision (Variables|Default|GetStrikeCollision))
  (bind _relativerotation (Variables|/Script/Engine.SceneComponent|GetRelativeRotation _hammer))
  (:Pressed
    (if (not (Audio|Components|Audio|IsPlaying (Variables|Default|GetHammerSwingTimeline)))
      (bind _swing (Timeline|HammerSwingTimeline PlayFromStart)
        (:Update
          (Transformation|SetRelativeRotation _hammer (Math|Rotator|MakeRotator (.roll _relativerotation) _swing (.yaw _relativerotation)) false false))
        (:HitBegin
          (Variables|/Script/Engine.PrimitiveComponent|SetbGenerateOverlapEvents _strikecollision true)
          (Audio|PlaySound2D "/Game/Assets/Audio/Swing.Swing" 1.0 1.0 0.0 0 0))
        (:HitEnd
          (Variables|/Script/Engine.PrimitiveComponent|SetbGenerateOverlapEvents _strikecollision false))))))

(event Input|AxisEvents|InputAxisForwardMovement
  (params (AxisValue :type Float%20%28single-precision%29))
  (Variables|Default|SetMovementInput (Math|Vector2D|MakeVector2D AxisValue (.y (Variables|Default|GetMovementInput)))))

(event Input|AxisEvents|InputAxisTurn
  (params (AxisValue :type Float%20%28single-precision%29))
  (Class|Actor|AddActorWorldRotation (Math|Rotator|MakeRotator 0.0 0.0 (* AxisValue (Class|GameplayStatics|GetGlobalTimeDilation)))))

(event Input|AxisEvents|InputAxisSideMovement
  (params (AxisValue :type Float%20%28single-precision%29))
  (Variables|Default|SetMovementInput (Math|Vector2D|MakeVector2D (.x (Variables|Default|GetMovementInput)) AxisValue)))

(fn ConstructionScript)