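; Game mode for a timed whack-a-mole game that runs the start, play and game-over flow with their widgets.
; Start and game-over screens freeze play through zero global time dilation, and StartGame restores it, starts music, shows the HUD and sets timers.
; A looping timer spawns a mole in a randomly chosen empty hole by shuffling all BP_Hole actors.
; When the game timer expires, GameOver stops music and passes the HUD's score to the end screen.
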(event Custom|SpawnMole
  (bind _outactors (Actor|GetAllActorsOfClass "/Game/Blueprints/BP_Hole.BP_Hole_C"))
  (Utilities|Array|Shuffle _outactors)
  (bind _array_element (Utilities|Array|ForEachLoopwithBreak _outactors :!label _label)
    (:LoopBody
      (if (not (Default|HasMole _array_element))
        (Default|SpawnMole _array_element)
        (goto _label Break)))))

(event Custom|GameOver
  (bind _hud (Variables|Default|GetHUD))
  (Audio|PlaySound2D "/Game/Assets/Audio/GameOver.GameOver" 1.0 1.0 0.0 0 0)
  (Audio|Components|Audio|Stop (Variables|Default|GetMusic))
  (Utilities|Time|SetGlobalTimeDilation 0.0)
  (Widget|RemovefromParent _hud)
  (bind _returnvalue (UserInterface|CreateWidget "/Game/Blueprints/WBP_GameOver.WBP_GameOver_C" (Game|GetPlayerController 0)))
  (Variables|/Game/Blueprints/WBP_GameOver.WBP_GameOver_C|SetScore _returnvalue (Variables|/Game/Blueprints/WBP_HUD.WBP_HUD_C|GetScore _hud))
  (UserInterface|Viewport|AddtoViewport _returnvalue 0))

(event Custom|StartGame
  (bind _gametime (Variables|Default|GetGameTime))
  (Utilities|Time|SetGlobalTimeDilation 1.0) ; Unpause Game
  (Audio|Components|Audio|Play (Variables|Default|GetMusic) 0.0)
  (bind _returnvalue (UserInterface|CreateWidget "/Game/Blueprints/WBP_HUD.WBP_HUD_C" (Game|GetPlayerController 0)))
  (bind _output_get (Variables|Default|SetHUD _returnvalue))
  (Variables|/Game/Blueprints/WBP_HUD.WBP_HUD_C|SetTimeLeft _output_get _gametime)
  (UserInterface|Viewport|AddtoViewport _output_get 0)
  (Utilities|Time|SetTimerbyEvent (delegate Custom|GameOver) _gametime)
  (Utilities|Time|SetTimerbyEvent (delegate Custom|SpawnMole) (Variables|Default|GetSpawnDelay) true false 1.0))

(event EventBeginPlay
  (bind _returnvalue (UserInterface|CreateWidget "/Game/Blueprints/WBP_StartScreen.WBP_StartScreen_C" (Game|GetPlayerController 0)))
  (UserInterface|Viewport|AddtoViewport _returnvalue 0)
  (Utilities|Time|SetGlobalTimeDilation 0.0))

(event EventTick
  (params (DeltaSeconds :type Float%20%28single-precision%29)))

(fn ConstructionScript)